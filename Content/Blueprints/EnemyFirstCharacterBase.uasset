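; Base enemy character that carries an axe, takes damage and dies, with a widget health bar.
; On BeginPlay it spawns a BaseAxe on the mesh's Axe socket and registers itself as the health widget's owner.
; Damage lowers health, then either plays an injury montage while toggling movement off, or a one-time death montage before destroying axe and enemy.
; TryAxeSwipe plays the attack montage.
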(event `self.ReceiveAnyDamage`
  (params (Damage :type "Float (single-precision)") (DamageType :type "DamageType Object Reference") (InstigatedBy :type "Controller Object Reference") (DamageCauser :type "Actor Object Reference"))
  (set `self.IsHurting` true)
  (bind _output_get (set `self.EnemyHealth` (- (`self.EnemyHealth`) Damage)))
  (if (<= _output_get 0.0)
    (set `self.IsDying` true)
    (`/Engine/EditorBlueprintResources/StandardMacros.DoOnce` false
      (:`Completed`
        (`CharacterMovementComponent.DisableMovement` (`self.CharacterMovement`))
        (bind _returnvalue (`self.PlayAnimMontage` "/Game/Blueprints/AM_EnemyFirstAnimDeath.AM_EnemyFirstAnimDeath"))
        (`KismetSystemLibrary.Delay` _returnvalue)
        (`self.K2_DestroyActor` (`self.MyNewAxe`))
        (`self.K2_DestroyActor`)))
    (else
      (`ActorComponent.ToggleActive` (`self.CharacterMovement`))
      (bind _returnvalue_2 (`self.PlayAnimMontage` "/Game/Blueprints/Animations/AM_EnemyInjury.AM_EnemyInjury"))
      (`KismetSystemLibrary.Delay` _returnvalue_2)
      (`ActorComponent.ToggleActive` (`self.CharacterMovement`))
      (set `self.IsHurting` false))))

(event `TryAxeSwipe`
  (`self.PlayAnimMontage` "/Game/Blueprints/Animations/AM_AttackRight.AM_AttackRight"))

(event `self.ReceiveBeginPlay`
  (`self.Create Axe`)
  (bind _ashealth_widget (cast `/Game/Blueprints/HealthWidget` (`WidgetComponent.GetUserWidgetObject` (`self.HealthBar`))))
  (`/Game/Blueprints/HealthWidget.SetOwningEnemy` _ashealth_widget self))

(event `Create Axe`
  (bind _returnvalue (`|SpawnActorFromClass` "/Game/Blueprints/BaseAxe.BaseAxe_C" (`self.GetTransform`) "Undefined" "OverrideRootScale" null null))
  (`self.K2_AttachToComponent` _returnvalue (`self.Mesh`) "Axe" "SnapToTarget" "SnapToTarget" "SnapToTarget" false)
  (set `self.MyNewAxe` _returnvalue))

(fn `NewFunction_0`
  (returns (`AsHealth Widget` :type "/Game/Blueprints/HealthWidget Object Reference") (ReturnValue :type "UserWidget Object Reference")))

(fn `UserConstructionScript`)