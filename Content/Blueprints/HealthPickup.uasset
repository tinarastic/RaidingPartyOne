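; HealthPickup is an actor that restores health to a Viking character that overlaps it.
; On overlap it casts to VikingCharacterBase and compares current Health with a value read from that character's class defaults, which serves as the maximum.
; If they differ, it adds HealthOffering capped at that value and destroys itself, so characters at full health leave the pickup in place.
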(event `self.ReceiveActorBeginOverlap`
  (params (OtherActor :type "Actor Object Reference"))
  (bind _asviking_character_base (cast `/Game/Blueprints/VikingCharacterBase` OtherActor))
  (bind _health (defaults `/Game/Blueprints/HealthPickup` (`GameplayStatics.GetObjectClass` _asviking_character_base)))
  (if (not (== _health (`/Game/Blueprints/VikingCharacterBase.Health` _asviking_character_base)))
    (set `/Game/Blueprints/VikingCharacterBase.Health` (`KismetMathLibrary.FMin` (+ (`/Game/Blueprints/VikingCharacterBase.Health` _asviking_character_base) (`self.Health offering`)) _health) _asviking_character_base)
    (`self.K2_DestroyActor`)))

(fn `UserConstructionScript`)