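; VikingGameMode is a game mode that runs waves of AI enemies, starting from the first on BeginPlay.
; Each wave copies its class list from Waves into a shuffled Queue.
; A looping timer spawns the queue's front class at a random PlayerStart, dequeuing it on success.
; Each spawn's OnDestroyed triggers a check that advances WaveIndex, without a bounds check, once the queue and EnemyAIControllerBase actors are gone.
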(event `self.ReceiveBeginPlay`
  (`KismetSystemLibrary.K2_SetTimerDelegate` (delegate `SpawnEnemy`) 5.0 true)
  (`self.ResetGame`))

(event `SpawnEnemy`
  (if (>= (`KismetArrayLibrary.Array_Length` (`self.Queue`)) 0)
    (bind _outactors (`GameplayStatics.GetAllActorsOfClass` "/Script/Engine.PlayerStart"))
    (bind _output (`|GetArrayItem` _outactors (`KismetMathLibrary.RandomInteger` (`KismetArrayLibrary.Array_Length` _outactors))))
    (bind _returnvalue (`AIBlueprintHelperLibrary.SpawnAIFromClass` (`|GetArrayItem` (`self.Queue`)) null (`self.K2_GetActorLocation` _output) (`self.K2_GetActorRotation` _output)))
    (`/Engine/EditorBlueprintResources/StandardMacros.IsValid` _returnvalue
      (:`Is Valid`
        (`KismetArrayLibrary.Array_Remove` (`self.Queue`))
        (add `self.OnDestroyed` _returnvalue (delegate `CheckWaveComplete`))))))

(event `CheckWaveComplete` :!signature `self.OnDestroyed`
  (params (DestroyedActor :type "Actor Object Reference"))
  (if (== (`KismetArrayLibrary.Array_Length` (`self.Queue`)) 0)
    (bind _outactors (`GameplayStatics.GetAllActorsOfClass` "/Game/Blueprints/EnemyAIControllerBase.EnemyAIControllerBase_C"))
    (if (== (`KismetArrayLibrary.Array_Length` _outactors) 0)
      (`self.StartNewWave`))))

(event `ResetGame`
  (bind _output_classtospawn (break `/Game/Blueprints/EnemySpawnStruct` (`|GetArrayItem` (`self.Waves`) (`self.WaveIndex`))))
  (set `self.WaveIndex` 0)
  (bind _output_get (set `self.Queue` _output_classtospawn :!label _label))
  (`KismetArrayLibrary.Array_Shuffle` _output_get))

(event `StartNewWave`
  (`/Engine/EditorBlueprintResources/StandardMacros.IncrementInt` (`self.WaveIndex`)
    (:`  `
      (goto _label))))

(fn `UserConstructionScript`)