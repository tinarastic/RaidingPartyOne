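; Base player controller that turns input into movement, jumping and a swipe attack for the controlled Viking pawn.
; The Up axis adds movement along the camera manager's up vector, while the Right axis turns via controller yaw input.
; Jump casts the pawn to Character, and SwipeAttack casts to VikingCharacterBase to play the swipe attack montage directly.
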(event `self.ReceiveTick`
  (params (DeltaSeconds :type "Float (single-precision)")))

(event `InputAction|Jump`
  (params (Key :type "Key Structure"))
  (bind _returnvalue (`self.K2_GetPawn`))
  (:`Pressed`
    (`/Engine/EditorBlueprintResources/StandardMacros.IsValid` _returnvalue
      (:`Is Valid`
        (bind _ascharacter (cast `Character` _returnvalue))
        (`Character.Jump` _ascharacter)))))

(event `InputAxis|Up`
  (params (AxisValue :type "Float (single-precision)"))
  (bind _returnvalue (`self.K2_GetPawn`))
  ;[1 1 1] Basic movements - forward/turn
  (`/Engine/EditorBlueprintResources/StandardMacros.IsValid` _returnvalue
    (:`Is Valid`
      (`Pawn.AddMovementInput` _returnvalue (`SceneComponent.GetUpVector` (`PlayerCameraManager.TransformComponent` (`self.PlayerCameraManager`))) AxisValue false))))

(event `InputAction|SwipeAttack`
  (params (Key :type "Key Structure"))
  (:`Pressed`
    (bind _asviking_character_base (cast `/Game/Blueprints/VikingCharacterBase` (`self.K2_GetPawn`)))
    (`Character.PlayAnimMontage` _asviking_character_base "/Game/Blueprints/AM_VikingSwipeAttack.AM_VikingSwipeAttack" 1.0 "None")))

(event `InputAxis|Right`
  (params (AxisValue :type "Float (single-precision)"))
  ;[1 1 1] Basic movements - forward/turn
  (`/Engine/EditorBlueprintResources/StandardMacros.IsValid` (`self.K2_GetPawn`)
    (:`Is Valid`
      (`self.AddYawInput` AxisValue))))

(fn `UserConstructionScript`)